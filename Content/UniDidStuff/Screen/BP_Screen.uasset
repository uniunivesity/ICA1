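; BP_Screen is a screen actor that shows a stay-nearby countup and announces a warp destination as acquired after five seconds.
; When the third-person character overlaps its Box, it records the contact time and plays the PlayerNextTo timeline, whose updates write elapsed seconds to a TextRender.
; At the threshold it changes the message and color, plays a success sound and stops the timeline.
; Leaving the box stops the timeline; no warp logic lives here.
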(event `self.Box.OnComponentBeginOverlap`
  (params (OverlappedComponent :type "PrimitiveComponent Object Reference") (OtherActor :type "Actor Object Reference") (OtherComp :type "PrimitiveComponent Object Reference") (OtherBodyIndex :type Integer) (bFromSweep :type Boolean) (SweepResult :type "HitResult Structure (by ref)"))
  (bind _returnvalue (`GameplayStatics.GetTimeSeconds`))
  (bind _textrender (`self.TextRender`))
  (cast `/Game/ThirdPerson/Blueprints/BP_ThirdPersonCharacter` OtherActor)
  (bind _output_get (set `self.MomentOfContact` _returnvalue))
  (`Timeline|PlayerNextTo` :!label _label
    (:`Update`
      (bind _returnvalue_2 (- _returnvalue _output_get))
      (`TextRenderComponent.K2_SetText` (`self.TextRender`) (`KismetTextLibrary.Conv_DoubleToText` _returnvalue_2 "HalfToEven" false true 1 324 1 1))
      (if (>= _returnvalue_2 5.0)
        (`TextRenderComponent.K2_SetText` _textrender (`|FormatText` "warp destination \naquired."))
        (`TextRenderComponent.SetTextRenderColor` _textrender (make `Color` 0 100))
        (`GameplayStatics.PlaySoundAtLocation` "/Game/Scenarios/BaseContent/Audio/S_Success_01.S_Success_01" (`SceneComponent.K2_GetComponentLocation` (`self.StaticMeshComponent`)) (struct) 1.0 1.0 0.0 null null null null)
        (goto _label :!via `Stop`)))))

(event `self.Box.OnComponentEndOverlap`
  (params (OverlappedComponent :type "PrimitiveComponent Object Reference") (OtherActor :type "Actor Object Reference") (OtherComp :type "PrimitiveComponent Object Reference") (OtherBodyIndex :type Integer))
  (cast `/Game/ThirdPerson/Blueprints/BP_ThirdPersonCharacter` OtherActor)
  (goto _label :!via `Stop`))

(fn `UserConstructionScript`)