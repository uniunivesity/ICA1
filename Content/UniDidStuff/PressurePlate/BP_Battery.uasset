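; BP_Battery is a battery actor Blueprint whose event logic is all disconnected from any entry event, so none of it runs.
; The unwired logic uses a Linetrace timeline to cast a short forward visibility trace from the MaybeIllBeTracer component on each update.
; The hit result switches the static mesh's constraint mode between XY plane and default, with debug prints.
; The construction script is empty.
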(fn `UserConstructionScript`)