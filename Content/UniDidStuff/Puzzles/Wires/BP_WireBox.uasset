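; Wire box puzzle actor, apparently work in progress, that lets the player grab cables with the mouse.
; AttemptWireGrab sphere-traces from the cursor, matches the hit against LeftSide's child components, and converts its first tag into a cable index.
; GrabWire plays a timeline that sets that cable's EndLocation to a cursor line-trace impact point on each update.
; ReleaseWire and LockInWire are empty stubs, and debug prints and trace drawing remain.
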(event `AttemptWireGrab`
  (bind (_worldlocation _worlddirection) (`PlayerController.DeprojectMousePositionToWorld` (`GameplayStatics.GetPlayerController` 0)))
  (bind _outhit (`KismetSystemLibrary.SphereTraceSingleForObjects` :`Start` _worldlocation :`End` (+ _worldlocation (* _worlddirection 500)) :`Radius` 5.0 :`ObjectTypes` (`|MakeArray` "ObjectTypeQuery2" :!type "EObjectTypeQuery Enum") :`DrawDebugType` "ForDuration" :`bIgnoreSelf` false :`DrawTime` 0.2))
  (for _array_element (`SceneComponent.GetChildrenComponents` (`self.LeftSide`) false)
    (bind (_bblockinghit _binitialoverlap _time _distance _location _impactpoint _normal _impactnormal _physmat _hitactor _hitcomponent) (`GameplayStatics.BreakHitResult` _outhit))
    (bind _returnvalue (`KismetStringLibrary.Conv_NameToString` (`|GetArrayItem` (`ActorComponent.ComponentTags` _hitcomponent))))
    (bind _returnvalue_2 (== _array_element _hitcomponent))
    (`KismetSystemLibrary.PrintString` (`KismetStringLibrary.Concat_StrStr` _returnvalue "---" (`KismetStringLibrary.Conv_BoolToString` _returnvalue_2)))
    (if _returnvalue_2
      (`|ExecutionSequence`
        (:`then_0`
          (break))
        (:`then_1`
          (`self.GrabWire` (`KismetStringLibrary.Conv_StringToInt` _returnvalue)))))))

(event `GrabWire`
  (params (GrabbedCable :type Integer))
  (bind (_worldlocation _worlddirection) (`PlayerController.DeprojectMousePositionToWorld` (`GameplayStatics.GetPlayerController` 0)))
  (bind _children (`SceneComponent.GetChildrenComponents` (`self.Cables`) false))
  (bind _ascable_component (cast `CableComponent` (`|GetArrayItem` _children GrabbedCable)))
  (`Timeline|UpdateWireEndPoint`
    (:`Update`
      (bind _outhit (`KismetSystemLibrary.LineTraceSingle` :`Start` _worldlocation :`End` (+ _worldlocation (* _worlddirection 500)) :`TraceChannel` "TraceTypeQuery1" :`DrawDebugType` "ForOneFrame" :`bIgnoreSelf` false))
      (set `CableComponent.EndLocation` (`.ImpactPoint` (`GameplayStatics.BreakHitResult` _outhit)) _ascable_component))))

(event `ReleaseWire`)

(event `LockInWire`)

(fn `UserConstructionScript`)