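; A single keypad key actor that acts as a number, Backspace or Enter button for its parent BP_KeyPad.
; The construction script sets the label and scale from ButtonType, keeping the extra mesh and collision only for Enter.
; PushButton sends the type and number to the parent's KeyPress, then gives press feedback with a temporary material swap and a short move of the text component out and back.
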(event `PushButton`
  (bind _buttontext (`self.ButtonText`))
  (bind _asbp_key_pad (cast `/Game/UniDidStuff/Puzzles/KeyPad/BP_KeyPad` (`self.GetParentActor` self)))
  (`/Game/UniDidStuff/Puzzles/KeyPad/BP_KeyPad.KeyPress` _asbp_key_pad (`self.ButtonType`) (`self.ButtonNumber`))
  (`PrimitiveComponent.SetMaterial` (`self.ButtonMesh`) 0 "/Game/Scenarios/BaseContent/Materials/Bases/M_TaskExitLighter.M_TaskExitLighter")
  (bind _buttonmeshextra (`self.ButtonMeshExtra`)
    (:`then`
      (`PrimitiveComponent.SetMaterial` _buttonmeshextra 0 "/Game/Scenarios/BaseContent/Materials/Bases/M_TaskExitLighter.M_TaskExitLighter"))
    (:`else`
      _))
  (`KismetSystemLibrary.MoveComponentTo` _buttontext (+ (`self.ReturnPos`) (-5.0 0.0 0.0)) (`SceneComponent.RelativeRotation` _buttontext) :!label _label)
  (`KismetSystemLibrary.MoveComponentTo` _buttontext (`self.ReturnPos`) (`SceneComponent.RelativeRotation` _buttontext))
  (`|ExecutionSequence`
    (:`then_0`
      (goto _label :!via `Return`))
    (:`then_1`
      (`PrimitiveComponent.SetMaterial` (`self.ButtonMesh`) 0 "/Game/Scenarios/BaseContent/Materials/Bases/M_SimpleFlatColour.M_SimpleFlatColour")
      (bind _buttonmeshextra_2 (`self.ButtonMeshExtra`)
        (:`then`
          (`PrimitiveComponent.SetMaterial` _buttonmeshextra_2 0 "/Game/Scenarios/BaseContent/Materials/Bases/M_SimpleFlatColour.M_SimpleFlatColour"))
        (:`else`)))))

(fn `BecomeBackspace`
  (bind _buttoncollision (`self.ButtonCollision`))
  (bind _buttonmesh (`self.ButtonMesh`))
  (`SceneComponent.SetRelativeScale3D` _buttonmesh (* (`SceneComponent.RelativeScale3D` _buttonmesh) (1.0 2.0 1.0)))
  (`SceneComponent.SetRelativeScale3D` _buttoncollision (* (`SceneComponent.RelativeScale3D` _buttoncollision) (1.0 2.0 1.0)))
  (`TextRenderComponent.K2_SetText` (`self.ButtonText`) (`|FormatText` "«")))

(fn `BecomeEnter`
  (bind _buttonmesh (`self.ButtonMesh`))
  (bind _buttoncollision (`self.ButtonCollision`))
  (`SceneComponent.SetRelativeScale3D` _buttonmesh (* (`SceneComponent.RelativeScale3D` _buttonmesh) (1.0 1.0 2.0)))
  (`SceneComponent.SetRelativeScale3D` _buttoncollision (* (`SceneComponent.RelativeScale3D` _buttoncollision) (1.0 1.0 2.0)))
  (`TextRenderComponent.K2_SetText` (`self.ButtonText`) (`|FormatText` "=")))

(fn `BecomeNumber`
  (`TextRenderComponent.K2_SetText` (`self.ButtonText`) (`KismetTextLibrary.Conv_IntToText` (`self.ButtonNumber`))))

(fn `UserConstructionScript`
  (if (`|EnumEquality` (`self.ButtonType`) "NewEnumerator2")
    (set `self.ReturnPos` (`SceneComponent.RelativeLocation` (`self.ButtonText`)) :!label _label)
    (switch `/Game/UniDidStuff/Puzzles/KeyPad/E_ButtonType` (`self.ButtonType`)
      (:`NewEnumerator0`
        (`self.BecomeNumber`))
      (:`NewEnumerator1`
        (`self.BecomeBackspace`))
      (:`NewEnumerator2`
        (`self.BecomeEnter`)))
    (else
      (`|ExecutionSequence`
        (:`then_0`
          (`ActorComponent.K2_DestroyComponent` (`self.ButtonCollisionExtra`))
          (`ActorComponent.K2_DestroyComponent` (`self.ButtonMeshExtra`)))
        (:`then_1`
          (goto _label))))))