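; Keypad puzzle actor with a text screen, where number, backspace and enter presses edit and check a typed code.
; A sphere trace from the mouse cursor finds and pushes BP_KeyPadButton actors, while KeyPress handles each button type.
; Input is length-capped with a red flash on overflow; Enter compares it to a hardcoded code, printing and flashing green on a match.
; The colour flash resets to white through a retriggerable delay.
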(event `ClickOnButtonsTrace`
  (bind (_worldlocation _worlddirection) (`PlayerController.DeprojectMousePositionToWorld` (`GameplayStatics.GetPlayerController` 0)))
  (bind _outhit (`KismetSystemLibrary.SphereTraceSingleForObjects` :`Start` _worldlocation :`End` (+ _worldlocation (* _worlddirection 500)) :`Radius` 5.0 :`ObjectTypes` (`|MakeArray` "ObjectTypeQuery2" :!type "EObjectTypeQuery Enum") :`bIgnoreSelf` false :`DrawTime` 0.2))
  (bind _asbp_key_pad_button (cast `/Game/UniDidStuff/Puzzles/KeyPad/BP_KeyPadButton` (`.HitActor` (`GameplayStatics.BreakHitResult` _outhit))))
  (`/Game/UniDidStuff/Puzzles/KeyPad/BP_KeyPadButton.PushButton` _asbp_key_pad_button))

(event `KeyPress`
  (params (ButtonType :type "/Game/UniDidStuff/Puzzles/KeyPad/E_ButtonType Enum" :default "NewEnumerator0") (ButtonNumber :type Integer))
  (switch `/Game/UniDidStuff/Puzzles/KeyPad/E_ButtonType` ButtonType
    (:`NewEnumerator0`
      (bind _addednumber (`self.AddNumberToScreen` 6 ButtonNumber))
      (if (not _addednumber)
        (`self.SetColourThenWhite` 0 0 255)))
    (:`NewEnumerator1`
      (`self.RemoveLastDigit`))
    (:`NewEnumerator2`
      (if (`KismetTextLibrary.EqualEqual_TextText` (`TextRenderComponent.Text` (`self.ScreenText`)) (`|FormatText` "69420"))
        (`KismetSystemLibrary.PrintString` "noway")
        (`self.SetColourThenWhite` 0 255)))))

(fn `AddNumberToScreen`
  (params (Max :type Integer) (ButtonNumber :type Integer))
  (returns (AddedNumber :type Boolean))
  (locals (AddedNum :type Boolean))
  (bind _screentext (`self.ScreenText`))
  (bind _returnvalue (`KismetTextLibrary.Conv_TextToString` (`TextRenderComponent.Text` _screentext)))
  (bind _output_get (set `local.AddedNum` (< (`KismetStringLibrary.Len` _returnvalue) Max)))
  (if _output_get
    (`TextRenderComponent.K2_SetText` _screentext (`KismetTextLibrary.Conv_StringToText` (`KismetStringLibrary.BuildString_Int` _returnvalue "" ButtonNumber))))
  (return (`local.AddedNum`)))

(fn `RemoveLastDigit`
  (bind _screentext (`self.ScreenText`))
  (`TextRenderComponent.K2_SetText` _screentext (`KismetTextLibrary.Conv_StringToText` (`KismetStringLibrary.LeftChop` (`KismetTextLibrary.Conv_TextToString` (`TextRenderComponent.Text` _screentext)) 1))))

(fn `UserConstructionScript`)