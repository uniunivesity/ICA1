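; Keycard pickup that grants BP_Rover HasKeycard when it overlaps the sphere, then plays a collection animation and destroys itself.
; The Anim timeline scales and spins the mesh, adds a height offset and pulls it toward the player pawn with a distance-scaled lerp, holding XY once close.
; After a short delay, Poof closes the gate on timeline-driven scaling so ScaleDown can shrink the mesh to zero before destroying the actor.
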(event `self.Sphere.OnComponentBeginOverlap`
  (params (OverlappedComponent :type "PrimitiveComponent Object Reference") (OtherActor :type "Actor Object Reference") (OtherComp :type "PrimitiveComponent Object Reference") (OtherBodyIndex :type Integer) (bFromSweep :type Boolean) (SweepResult :type "HitResult Structure (by ref)"))
  (bind _staticmeshcomponent (`self.StaticMeshComponent`))
  (bind _returnvalue (`self.K2_GetActorLocation` (`GameplayStatics.GetPlayerPawn` 0)))
  (bind _returnvalue_2 (`SceneComponent.K2_GetComponentLocation` _staticmeshcomponent))
  (bind (_returnvalue_x _returnvalue_y) (`KismetMathLibrary.BreakVector` (`SceneComponent.K2_GetComponentLocation` _staticmeshcomponent)))
  (bind (_returnvalue_roll _returnvalue_pitch _returnvalue_yaw) (`KismetMathLibrary.BreakRotator` (`SceneComponent.K2_GetComponentRotation` _staticmeshcomponent)))
  (bind _returnvalue_3 (`KismetMathLibrary.Vector_Distance` _returnvalue_2 _returnvalue))
  (bind (_returnvalue_x_2 _returnvalue_y_2 _returnvalue_z) (`KismetMathLibrary.BreakVector` (`KismetMathLibrary.VLerp` _returnvalue_2 _returnvalue (* _returnvalue_3 0.0001))))
  (bind _asbp_rover (cast `/Game/UniDidStuff/Player/BP_Rover` OtherActor))
  (set `/Game/UniDidStuff/Player/BP_Rover.HasKeycard` true _asbp_rover)
  (`|ExecutionSequence`
    (:`then_0`
      (`KismetSystemLibrary.Delay` 2.0)
      (`self.Poof`))
    (:`then_1`
      (bind (_direction _scale _hieght) (`Timeline|Anim`)
        (:`Update`
          (`|ExecutionSequence`
            (:`then_0`
              (`/Engine/EditorBlueprintResources/StandardMacros.Gate` false :!label _label
                (:`Exit`
                  (`SceneComponent.SetRelativeScale3D` _staticmeshcomponent (`KismetMathLibrary.Conv_DoubleToVector` _scale)))))
            (:`then_1`
              (`SceneComponent.K2_SetRelativeRotation` _staticmeshcomponent (`KismetMathLibrary.MakeRotator` _returnvalue_roll _returnvalue_pitch (+ _returnvalue_yaw 5.0)) false false))
            (:`then_2`
              (if (<= _returnvalue_3 100.0)
                (bind _returnvalue_4 (+ _hieght _returnvalue_z))
                (`SceneComponent.K2_SetRelativeLocation` _staticmeshcomponent (`KismetMathLibrary.MakeVector` _returnvalue_x _returnvalue_y _returnvalue_4) false false)
                (else
                  (`SceneComponent.K2_SetRelativeLocation` _staticmeshcomponent (`KismetMathLibrary.MakeVector` _returnvalue_x_2 _returnvalue_y_2 _returnvalue_4) false false))))))))))

(event `Poof`
  (bind _relativescale3d (`SceneComponent.RelativeScale3D` (`self.StaticMeshComponent`)))
  (`|ExecutionSequence`
    (:`then_0`
      (goto _label :!via `Close`))
    (:`then_1`
      (`Timeline|ScaleDown`
        (:`Update`
          (`SceneComponent.SetRelativeScale3D` (`self.StaticMeshComponent`) (- _relativescale3d (0.015 0.015 0.015)))
          (if (<= (.z _relativescale3d) 0.0)
            (`KismetSystemLibrary.PrintString` "goodbye cruel world" :!label _label_2)
            (`self.K2_DestroyActor`)))
        (:`Finished`
          (goto _label_2))))))

(fn `UserConstructionScript`)