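; BP_DoorMultiInput is a door that opens once its accumulated power reaches RequiredPower and closes when it drops below.
; UpdatePower adds a signed difference to Power, refreshes the indicators, then slides Cover along Y from the closed position captured in the construction script, or back to it.
; Children of Lights turn green up to the Power count and red beyond it.
; Tick prints Power as debug output.
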(event `Open`
  (bind _cover (`self.Cover`))
  (`KismetSystemLibrary.MoveComponentTo` _cover (- (`self.ClosedPos`) (0.0 300.0 0.0)) (`SceneComponent.RelativeRotation` _cover) true false 1.0))

(event `UpdatePower`
  (params (PowerDifference :type Integer))
  (bind _output_get (set `self.Power` (+ PowerDifference (`self.Power`))))
  (`self.UpdateLights`)
  (if (>= _output_get (`self.RequiredPower`))
    (`self.Open`)
    (else
      (`self.Close`))))

(event `Close`
  (bind _cover (`self.Cover`))
  (`KismetSystemLibrary.MoveComponentTo` _cover (`self.ClosedPos`) (`SceneComponent.RelativeRotation` _cover) true false 1.0))

(event `UpdateLights`
  (for (_array_element _array_index) (`SceneComponent.GetChildrenComponents` (`self.Lights`) false)
    (bind _asprimitive_component (cast `PrimitiveComponent` _array_element))
    (`PrimitiveComponent.SetMaterial` _asprimitive_component 0 (select `bool` (<= (+ _array_index 1) (`self.Power`)) :`false` "/Game/UniDidStuff/Puzzles/Wires/MAT_PlasicWire_Red.MAT_PlasicWire_Red" :`true` "/Game/UniDidStuff/Puzzles/Wires/MAT_PlasicWire_Green.MAT_PlasicWire_Green" :!type "MaterialInterface Object Reference"))))

(event `self.ReceiveTick`
  (params (DeltaSeconds :type "Float (single-precision)"))
  (`KismetSystemLibrary.PrintString` (`KismetStringLibrary.Conv_IntToString` (`self.Power`)) true false (struct :`G` 0.66 :`B` 1.0 :`A` 1.0) 2.0 "fasedgta"))

(fn `UserConstructionScript`
  (set `self.ClosedPos` (`SceneComponent.RelativeLocation` (`self.Cover`))))