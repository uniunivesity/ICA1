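; BP_DoorButton is a door-related actor that plays a denied sound when the third-person character overlaps its trigger, as long as its gate is open.
; The MoveBrah event closes that gate, silencing further denial sounds, and eases the static mesh to an offset position and rotation in under a second.
; The move target is built from the mesh's world location but passed as a relative location.
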(event `self.Trigger.OnComponentBeginOverlap`
  (params (OverlappedComponent :type "PrimitiveComponent Object Reference") (OtherActor :type "Actor Object Reference") (OtherComp :type "PrimitiveComponent Object Reference") (OtherBodyIndex :type Integer) (bFromSweep :type Boolean) (SweepResult :type "HitResult Structure (by ref)"))
  (`KismetSystemLibrary.IsObjectOfSoftClass` OtherActor "/Game/ThirdPerson/Blueprints/BP_ThirdPersonCharacter.BP_ThirdPersonCharacter_C"
    (:`True`
      (`/Engine/EditorBlueprintResources/StandardMacros.Gate` false :!label _label
        (:`Exit`
          (`GameplayStatics.PlaySoundAtLocation` "/Game/Scenarios/BaseContent/Audio/S_Denied_02.S_Denied_02" (`SceneComponent.K2_GetComponentLocation` (`self.StaticMeshComponent`)) (struct) 1.0 1.0 0.0 null null null null))))))

(event `MoveBrah`
  (`|ExecutionSequence`
    (:`then_0`
      (goto _label :!via `Close`))
    (:`then_1`
      (`KismetSystemLibrary.MoveComponentTo` (`self.StaticMeshComponent`) (- (`SceneComponent.K2_GetComponentLocation` (`self.StaticMeshComponent`)) (-500.0 0.0 0.0)) (struct :`Yaw` 90.0) true true 0.8))))

(fn `UserConstructionScript`)