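; BP_HangingJoltingCable is a hanging electrical cable hazard that jerks around at random and damages actors touching its loose end.
; On a randomly timed loop, Jolt pins the cable end to a random JoltPoints child for one tick, then releases it to swing freely.
; A sphere attached to the CableEnd socket applies damage on overlap.
; Both jolts and overlaps spawn an electric Niagara effect at the sphere.
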(event `ZipZap`
  (`NiagaraFunctionLibrary.SpawnSystemAtLocation` "/Game/UniDidStuff/DamageSources/NS_Electric.NS_Electric" (`SceneComponent.K2_GetComponentLocation` (`self.Sphere`))))

(event `self.ReceiveBeginPlay`
  (`KismetSystemLibrary.Delay` (`KismetMathLibrary.RandomFloatInRange` 0.0 2.0))
  (`self.Jolt`)
  (`KismetSystemLibrary.Delay` (`KismetMathLibrary.RandomFloatInRange` 2.0 7.0) :!label _label)
  (`self.Jolt`)
  (goto _label))

(event `Jolt`
  (bind _cable (`self.Cable`))
  (bind _outitem (`KismetArrayLibrary.Array_Random` (`SceneComponent.GetChildrenComponents` (`self.JoltPoints`) false)))
  (`CableComponent.SetAttachEndToComponent` _cable _outitem "None")
  (set `CableComponent.bAttachEnd` true _cable)
  (`KismetSystemLibrary.DelayUntilNextTick`)
  (set `CableComponent.bAttachEnd` false _cable)
  (`self.ZipZap`))

(event `self.Sphere.OnComponentBeginOverlap`
  (params (OverlappedComponent :type "PrimitiveComponent Object Reference") (OtherActor :type "Actor Object Reference") (OtherComp :type "PrimitiveComponent Object Reference") (OtherBodyIndex :type Integer) (bFromSweep :type Boolean) (SweepResult :type "HitResult Structure (by ref)"))
  (`GameplayStatics.ApplyDamage` OtherActor 25.0 null self)
  (`self.ZipZap`))

(fn `UserConstructionScript`
  (`SceneComponent.K2_AttachToComponent` (`self.Sphere`) (`self.Cable`) "CableEnd" "KeepRelative" "KeepRelative" "KeepRelative" true))