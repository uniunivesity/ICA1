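; BP_Globe is an interactive globe that animates and displays its rounded yaw while the player pawn is inside its sphere.
; On overlap, the RotateBrah timeline resumes from the current yaw to spin and bob the globe, turning the text toward the BP_Rover camera.
; A Scale timeline resizes the globe and toggles text visibility midway, reversing on exit as rotation stops.
; An event track refreshes the number, which the construction script initializes.
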(event `self.Sphere.OnComponentBeginOverlap`
  (params (OverlappedComponent :type "PrimitiveComponent Object Reference") (OtherActor :type "Actor Object Reference") (OtherComp :type "PrimitiveComponent Object Reference") (OtherBodyIndex :type Integer) (bFromSweep :type Boolean) (SweepResult :type "HitResult Structure (by ref)"))
  (bind _textrender (`self.TextRender`))
  (bind (_relativerotation_roll _relativerotation_pitch _relativerotation_yaw) (`KismetMathLibrary.BreakRotator` (`SceneComponent.RelativeRotation` (`self.globe`))))
  (bind (_relativerotation_roll_2 _relativerotation_pitch_2 _relativerotation_yaw_2) (`KismetMathLibrary.BreakRotator` (`SceneComponent.RelativeRotation` (`self.globe`))))
  (if (== OtherActor (`GameplayStatics.GetPlayerPawn` 0))
    (`|ExecutionSequence`
      (:`then_0`
        (bind (_direction _bobbing _rotation) (`Timeline|RotateBrah` :`NewTime` (* (/ (+ _relativerotation_yaw_2 180.0) 360.0) 4.0) :!via `SetNewTime` :!label _label)
          (:`Update`
            (`SceneComponent.K2_SetRelativeLocationAndRotation` (`self.globe`) (`KismetMathLibrary.MakeVector` 0.0 0.0 _bobbing) (`KismetMathLibrary.MakeRotator` 0.0 0.0 _rotation) false false)
            (bind _asbp_rover (cast `/Game/UniDidStuff/Player/BP_Rover` (`GameplayStatics.GetPlayerPawn` 0)))
            (`SceneComponent.K2_SetRelativeRotation` _textrender (`KismetMathLibrary.FindLookAtRotation` (`SceneComponent.K2_GetComponentLocation` _textrender) (`SceneComponent.K2_GetComponentLocation` (`/Game/UniDidStuff/Player/BP_Rover.Camera` _asbp_rover))) false false))
          (:`Change text when hidden`
            (`TextRenderComponent.K2_SetText` (`self.TextRender`) (`KismetTextLibrary.Conv_IntToText` (* (`KismetMathLibrary.Round` (/ _relativerotation_yaw 10.0)) 10))))))
      (:`then_1`
        (goto _label))
      (:`then_2`
        (bind (_direction_2 _heyyy) (`Timeline|Scale` :!label _label_2)
          (:`Update`
            (`SceneComponent.SetRelativeScale3D` (`self.globe`) (`KismetMathLibrary.Conv_DoubleToVector` _heyyy)))
          (:`Halfway`
            (`SceneComponent.SetVisibility` (`self.TextRender`) (`|EnumEquality` _direction_2 "Forward") false)))))))

(event `self.Sphere.OnComponentEndOverlap`
  (params (OverlappedComponent :type "PrimitiveComponent Object Reference") (OtherActor :type "Actor Object Reference") (OtherComp :type "PrimitiveComponent Object Reference") (OtherBodyIndex :type Integer))
  (if (== (`GameplayStatics.GetPlayerPawn` 0) OtherActor)
    (`|ExecutionSequence`
      (:`then_0`
        (goto _label :!via `Stop`))
      (:`then_1`
        (goto _label_2 :!via `Reverse`)))))

(fn `UserConstructionScript`
  (bind (_relativerotation_roll _relativerotation_pitch _relativerotation_yaw) (`KismetMathLibrary.BreakRotator` (`SceneComponent.RelativeRotation` (`self.globe`))))
  (`TextRenderComponent.K2_SetText` (`self.TextRender`) (`KismetTextLibrary.Conv_IntToText` (* (`KismetMathLibrary.Round` (/ _relativerotation_yaw 10.0)) 10))))