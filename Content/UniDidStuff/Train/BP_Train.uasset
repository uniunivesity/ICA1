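; BP_Train is a train actor whose Body shuttles back and forth along world X or Y each time MoveMyJitty is called.
; Each call flips between the forward and backward arrows and line traces from the active one to measure travel distance, with debug drawing.
; The forward arrow's direction picks the axis.
; Paired eased MoveComponentTo nodes apply the offset, stopping one move and starting the opposite.
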(event `MoveMyJitty`
  (bind _body (`self.Body`))
  (bind (_returnvalue_x _returnvalue_y _returnvalue_z) (`KismetMathLibrary.BreakVector` (`SceneComponent.K2_GetComponentLocation` _body)))
  (bind _returnvalue (`SceneComponent.K2_GetComponentRotation` _body))
  (bind _returnvalue_x_2 (`KismetMathLibrary.BreakVector` (`SceneComponent.GetForwardVector` (`self.ArrowForward`))))
  (bind _output (`|GetArrayItem` (`|MakeArray` (`self.ArrowForward`) (`self.ArrowBackward`)) (`self.WhichArrow`)))
  (bind _returnvalue_2 (> _returnvalue_x_2 0.75))
  (bind _returnvalue_3 (`SceneComponent.K2_GetComponentLocation` _output))
  (bind _returnvalue_4 (`KismetMathLibrary.SelectFloat` _returnvalue_x _returnvalue_y _returnvalue_2))
  (bind _returnvalue_5 (`KismetSystemLibrary.MakeLiteralBool` (== (`self.WhichArrow`) 1)))
  (if _returnvalue_5
    (set `self.WhichArrow` 0)
    (else
      (set `self.WhichArrow` 1)))
  (bind _outhit (`KismetSystemLibrary.LineTraceSingle` :`Start` _returnvalue_3 :`End` (+ _returnvalue_3 (* (`SceneComponent.GetForwardVector` _output) 5000)) :`TraceChannel` "TraceTypeQuery1" :`DrawDebugType` "ForDuration"))
  (if _returnvalue_5
    (`|ExecutionSequence`
      (:`then_0`
        (goto _label_2 :!via `Stop`))
      (:`then_1`
        (bind (_bblockinghit _binitialoverlap _time _distance) (`GameplayStatics.BreakHitResult` _outhit))
        (bind _returnvalue_6 (+ _distance _returnvalue_4))
        (`KismetSystemLibrary.MoveComponentTo` _body (`KismetMathLibrary.MakeVector` (`KismetMathLibrary.SelectFloat` _returnvalue_6 _returnvalue_x _returnvalue_2) (`KismetMathLibrary.SelectFloat` _returnvalue_y _returnvalue_6 _returnvalue_2) _returnvalue_z) _returnvalue true true 2.5 :!label _label)))
    (else
      (`|ExecutionSequence`
        (:`then_0`
          (goto _label :!via `Stop`))
        (:`then_1`
          (bind _returnvalue_7 (- _returnvalue_4 _distance))
          (`KismetSystemLibrary.MoveComponentTo` _body (`KismetMathLibrary.MakeVector` (`KismetMathLibrary.SelectFloat` _returnvalue_7 _returnvalue_x _returnvalue_2) (`KismetMathLibrary.SelectFloat` _returnvalue_y _returnvalue_7 _returnvalue_2) _returnvalue_z) _returnvalue true true 2.5 :!label _label_2))))))

(fn `UserConstructionScript`)